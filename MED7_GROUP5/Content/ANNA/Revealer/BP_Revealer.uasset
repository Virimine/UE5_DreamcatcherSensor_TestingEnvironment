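; BP_Revealer is a pawn steered by normalized gyro values from an OSC receiver.
; Every tick, inverted gyro X drives movement input along the actor's forward vector and inverted gyro Y along its up vector.
; It then resets its location with X and Z clamped between min and max offsets, leaving Y unchanged.
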(event `self.ReceiveTick`
  (params (DeltaSeconds :type "Float (single-precision)"))
  (`self.AddMovementInput` (+ (* (`self.GetActorForwardVector`) (* (`/Game/ANNA/Revealer/Revealer_OSC_Component.NormGyroX` (`self.OSC_Receiver`)) -1.0)) (* (* (`/Game/ANNA/Revealer/Revealer_OSC_Component.NormGyroY` (`self.OSC_Receiver`)) -1.0) (`self.GetActorUpVector`))))
  (`self.K2_SetActorLocation` (`KismetMathLibrary.MakeVector` (`KismetMathLibrary.FClamp` (.x (`self.K2_GetActorLocation`)) (`self.MinOffsetX`) (`self.MaxOffsetX`)) (.y (`self.K2_GetActorLocation`)) (`KismetMathLibrary.FClamp` (.z (`self.K2_GetActorLocation`)) (`self.MinOffsetZ`) (`self.MaxOffsetZ`)))))

(fn `UserConstructionScript`)