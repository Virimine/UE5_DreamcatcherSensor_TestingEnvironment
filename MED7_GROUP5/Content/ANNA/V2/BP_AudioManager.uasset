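; BP_AudioManager plays a queue of up to five voice-over sounds in sequence through a single audio component.
; PlayVoiceOvers starts the first sound, and each OnAudioFinished advances a counter to play the next after a one-second delay.
; When the queue ends, it resets the counter and fires either a choice or narrative voice-over finished dispatcher, depending on the IsChoiceDialogue flag, with debug prints.
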(event `PlayVoiceOvers`
  (params (SoundsInQueue :type Integer) (NewSound :type "SoundBase Object Reference") (NewSound2 :type "SoundBase Object Reference") (NewSound3 :type "SoundBase Object Reference") (NewSound4 :type "SoundBase Object Reference") (NewSound5 :type "SoundBase Object Reference") (isChoiceDialogue :type Boolean))
  (`self.PlaySound` NewSound))

(event `self.Audio.OnAudioFinished`
  (bind _selection (`self.Selection`))
  (bind _result (`/Engine/EditorBlueprintResources/StandardMacros.IncrementInt` _selection)
    (:`  `
      (if (<= _selection (stale `PlayVoiceOvers` SoundsInQueue))
        (switch `int` _result
          (:`1`
            (`KismetSystemLibrary.Delay` 1.0)
            (`self.PlaySound` (stale `PlayVoiceOvers` NewSound2)))
          (:`2`
            (`KismetSystemLibrary.Delay` 1.0)
            (`self.PlaySound` (stale `PlayVoiceOvers` NewSound3)))
          (:`3`
            (`KismetSystemLibrary.Delay` 1.0)
            (`self.PlaySound` (stale `PlayVoiceOvers` NewSound4)))
          (:`4`
            (`KismetSystemLibrary.Delay` 1.0)
            (`self.PlaySound` (stale `PlayVoiceOvers` NewSound5))))
        (else
          (set `self.Selection` 0)
          (if (stale `PlayVoiceOvers` isChoiceDialogue)
            (`self.OnChoiceVoiceOverFinished`)
            (`KismetSystemLibrary.PrintString` "Exiting Chocie VoiceOver" true true (struct :`G` 0.66 :`B` 1.0 :`A` 1.0) 5.0)
            (else
              (`self.OnNarrativeVoiceOverFinished`)
              (`KismetSystemLibrary.PrintString` "Exiting NarrativeVoice Over" true true (struct :`G` 0.66 :`B` 1.0 :`A` 1.0) 5.0))))))))

(fn `UserConstructionScript`)